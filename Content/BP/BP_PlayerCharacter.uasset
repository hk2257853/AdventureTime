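; Player character Blueprint that serves as the UI layer for character interactions and quests.
; BeginPlay creates a persistent quest widget, which is refreshed when the quest list updates.
; OnShowUI creates the player widget on demand with Game and UI input, and OnHideUI returns it to parent and clears the reference.
; While that widget exists, events forward quest info and completion messages to it.
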(event `self.OnShowUI`
  (params (Character :type Name))
  (bind _returnvalue (`GameplayStatics.GetPlayerController` 0))
  (if (not (`KismetSystemLibrary.IsValid` (`self.PlayerUI`)))
    (bind _returnvalue_2 (`|CreateWidget` "/Game/Quest/UI/WBP_PlayerUI.WBP_PlayerUI_C" _returnvalue))
    (`WidgetBlueprintLibrary.SetInputMode_GameAndUIEx` _returnvalue _returnvalue_2)
    (`UserWidget.AddToViewport` _returnvalue_2 0)
    (bind _output_get (set `self.PlayerUI` _returnvalue_2))
    (`/Game/Quest/UI/WBP_PlayerUI.ShowUI` _output_get (`KismetTextLibrary.Conv_NameToText` Character))))

(event `self.OnHideUI`
  (bind _playerui (`self.PlayerUI`))
  (if (`KismetSystemLibrary.IsValid` _playerui)
    (`UINavWidget.ReturnToParent` _playerui false 0)
    (set `self.PlayerUI` null)))

(event `self.OnShowQuestInfo`
  (params (Quest :type "Quest Structure"))
  (bind _playerui (`self.PlayerUI`))
  ;[1 0.4784 0.5765] Show Quest Info
  (if (`KismetSystemLibrary.IsValid` _playerui)
    (`/Game/Quest/UI/WBP_PlayerUI.ShowQuestInfo` _playerui Quest_Message Quest_ItemQuestTexture)
    (else
      (`KismetSystemLibrary.PrintString` "Hello"))))

(event `self.OnShowQuestCompleted`
  (params (Message :type "Text (by ref)"))
  (bind _playerui (`self.PlayerUI`))
  ;[1 0.4784 0.5765] Show Quest completed
  (if (`KismetSystemLibrary.IsValid` _playerui)
    (`/Game/Quest/UI/WBP_PlayerUI.ShowQuestCompleted` _playerui Message)))

(event `self.ReceiveBeginPlay`
  ;[1 0.4784 0.5765] Quest UI
  (bind _returnvalue (`|CreateWidget` "/Game/Quest/UI/WBP_Quest.WBP_Quest_C" (`GameplayStatics.GetPlayerController` 0)))
  (`UserWidget.AddToViewport` _returnvalue 0)
  (set `self.QuestUI` _returnvalue))

(event `self.OnShowUpdatedQuestList`
  (params (QuestTextList :type "Array of Text (by ref)"))
  (bind _questui (`self.QuestUI`))
  ;[1 0.4784 0.5765] Quest UI
  (if (`KismetSystemLibrary.IsValid` _questui)
    (`/Game/Quest/UI/WBP_Quest.UpdateQuestList` _questui QuestTextList)))

(fn `UserConstructionScript`)